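; BP_Map is the tile map that tracks ship positions and answers neighbour queries for movement between BP_Tile actors.
; InitTiles caches every BP_Tile in MapList and has each one search for nearby tiles within a fixed distance.
; GetShipTile linearly scans that list for a ship's tile, feeding GetNextShipTile's directional lookup and NearOtherShip's check for an adjacent ship.
; Its event graph is empty, so all functions rely on external calls.
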(fn `Get Next Ship Tile`
  (params (Ship :type "/Game/BP/Entities/BP_Ship Object Reference") (Direction :type "/Game/Enum/Direction Enum" :default "NewEnumerator0"))
  (returns (Tile :type "/Game/BP/BP_Tile Object Reference") (TileExists :type Boolean))
  (bind (_tile _tile_exists) (`/Game/BP/BP_Tile.Get Direction Tile` (`self.GetShipTile` Ship) Direction))
  (return _tile _tile_exists))

(fn `GetShipTile`
  (params (Ship :type "/Game/BP/Entities/BP_Ship Object Reference"))
  (returns (Tile :type "/Game/BP/BP_Tile Object Reference"))
  (locals (FoundedShip :type "/Game/BP/BP_Tile Object Reference"))
  (for _array_element (`self.MapList`)
    (if (== (`/Game/BP/BP_Tile.ShipOnTile` _array_element) Ship)
      (return _array_element))))

(fn `InitTiles`
  (bind _outactors (`GameplayStatics.GetAllActorsOfClass` "/Game/BP/BP_Tile.BP_Tile_C"))
  (bind _output_get (set `self.MapList` _outactors))
  (for _array_element _output_get
    (`/Game/BP/BP_Tile.SearchNearTiles` _array_element 150.0)))

(fn `NearOtherShip`
  (params (Ship :type "/Game/BP/Entities/BP_Ship Object Reference") (Direction :type "/Game/Enum/Direction Enum" :default "NewEnumerator0"))
  (returns (`Ship In Direction` :type "/Game/BP/Entities/BP_Ship Object Reference") (`Exists an other Ship` :type Boolean))
  (bind (_tile _tileexists) (`self.Get Next Ship Tile` Ship Direction))
  (bind (_has_ship _ship) (`/Game/BP/BP_Tile.Has Ship` _tile))
  (if _tileexists
    (return _ship _has_ship)))

(fn `UserConstructionScript`)