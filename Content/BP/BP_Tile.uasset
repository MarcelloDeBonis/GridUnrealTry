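; BP_Tile is a board tile that tracks the ship on it and links to its four neighboring tiles.
; On BeginPlay it caches a child actor's world location as the ship position.
; SearchNearTiles stores neighbors found at a given distance, checking forward, right, left and back in a nested chain that stops at the first miss.
; Other functions return neighbors by direction and set, clear or report the occupying ship.
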(event `self.ReceiveBeginPlay`
  (`self.SetShipPosition`))

(fn `ArriveNewShip`
  (params (NewShip :type "/Game/BP/Entities/BP_Ship Object Reference"))
  (set `self.ShipOnTile` NewShip))

(fn `Get Direction Tile`
  (params (Direction :type "/Game/Enum/Direction Enum" :default "NewEnumerator0"))
  (returns (Tile :type "/Game/BP/BP_Tile Object Reference") (`Tile Exists` :type Boolean))
  (bind _righttile (`self.RightTile`))
  (bind _lefttile (`self.LeftTile`))
  (bind _backtile (`self.BackTile`))
  (bind _forwardtile (`self.ForwardTile`))
  (switch `/Game/Enum/Direction` Direction
    (:`NewEnumerator0`
      (return _forwardtile (`KismetSystemLibrary.IsValid` _forwardtile)))
    (:`NewEnumerator1`
      (return _righttile (`KismetSystemLibrary.IsValid` _righttile)))
    (:`NewEnumerator2`
      (return _lefttile (`KismetSystemLibrary.IsValid` _lefttile)))
    (:`NewEnumerator3`
      (return _backtile (`KismetSystemLibrary.IsValid` _backtile)))))

(fn `Has Ship`
  (returns (`Has Ship` :type Boolean) (Ship :type "/Game/BP/Entities/BP_Ship Object Reference"))
  (bind _shipontile (`self.ShipOnTile`))
  (return (!= _shipontile (`self.NoShip`)) _shipontile))

(fn `SearchNearTiles`
  (params (Distance :type "Float (double-precision)"))
  (locals (Direction :type "Vector Structure"))
  (bind (_founded _asbp_tile) (`/Game/Libraries/TileSearcher.Get Forward Tile` self Distance))
  (bind (_founded_2 _asbp_tile_2) (`/Game/Libraries/TileSearcher.GetRightTile` self Distance))
  (bind (_founded_3 _asbp_tile_3) (`/Game/Libraries/TileSearcher.GetLeftTile` self Distance))
  (bind (_founded_4 _asbp_tile_4) (`/Game/Libraries/TileSearcher.Get Back Tile` self Distance))
  (if _founded
    (set `self.ForwardTile` _asbp_tile)
    (if _founded_2
      (set `self.RightTile` _asbp_tile_2)
      (if _founded_3
        (set `self.LeftTile` _asbp_tile_3)
        (if _founded_4
          (set `self.BackTile` _asbp_tile_4)
          (return))))))

(fn `SetShipPosition`
  (set `self.ShipPosition` (`SceneComponent.K2_GetComponentLocation` (`self.ChildActor`))))

(fn `Ship Go`
  (set `self.ShipOnTile` (`self.NoShip`)))

(fn `UserConstructionScript`)