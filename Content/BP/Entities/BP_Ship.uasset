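; BP_Ship is a ship entity that moves tile to tile on BP_Map and takes damage.
; MoveCharacter asks the map whether the next tile in a direction exists and is free of other ships, then calls Move.
; Move lerps the actor's location on a timeline fed by distance over speed.
; TakeDamage subtracts from Life in the Stat struct and calls Die at zero or below, though Die and Attack are empty stubs.
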(event `Move`
  (params (Start :type "Vector Structure") (End :type "Vector Structure") (Speed :type "Float (double-precision)"))
  (bind (_direction _alpha) (`Timeline|MoveTimeline` :`NewTime` (/ (`KismetMathLibrary.VSize` (- End Start)) Speed))
    (:`Update`
      (`self.K2_SetActorLocation` (`KismetMathLibrary.VLerp` Start End _alpha)))))

(fn `Attack`
  (params (Direction :type "/Game/Enum/Direction Enum" :default "NewEnumerator0")))

(fn `Die`)

(fn `IsDied?`
  (returns (Died :type Boolean))
  (bind (_stat_team _stat_life) (break `/Game/Struct/ShipStat` (`self.Stat`)))
  (return (<= _stat_life 0)))

(fn `MoveCharacter`
  (params (Direction :type "/Game/Enum/Direction Enum" :default "NewEnumerator0"))
  (bind _outactors (`GameplayStatics.GetAllActorsOfClass` "/Game/BP/BP_Map.BP_Map_C"))
  (bind _output (`|GetArrayItem` _outactors))
  (bind (_tile _tileexists) (`/Game/BP/BP_Map.Get Next Ship Tile` _output self Direction))
  (if (and (not (`.Exists an other Ship` (`/Game/BP/BP_Map.NearOtherShip` _output self Direction))) _tileexists)
    (`self.Move` (`/Game/BP/BP_Tile.ShipPosition` (`/Game/BP/BP_Map.GetShipTile` _output self)) (`/Game/BP/BP_Tile.ShipPosition` _tile) 10.0)))

(fn `TakeDamage`
  (params (Damage :type Integer))
  (bind (_stat_team _stat_life _stat_attack _stat_shield _stat_percentageattack) (break `/Game/Struct/ShipStat` (`self.Stat`)))
  (set `self.Stat` (make `/Game/Struct/ShipStat` "NewEnumerator2" (- _stat_life Damage) _stat_attack _stat_shield _stat_percentageattack))
  (if (`self.IsDied?`)
    (`self.Die`)))

(fn `UserConstructionScript`)